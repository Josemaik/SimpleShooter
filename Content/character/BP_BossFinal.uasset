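; BP_BossFinal is the final boss character, with a health bar and a temporary electro-field shell.
; It tints the LifeBar widget cyan on BeginPlay, updates its percent from GetHealthPercent every Tick, and hides it at zero health.
; The shell mesh is hidden on possession.
; ActiveShell shows it for five seconds, then RemoveShell hides it and removes the "Shell" tag, which is not added in this Blueprint.
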(event `self.ReceiveBeginPlay`
  (bind _aswbp_life_bar_enemie (cast `/Game/UI/WBP_LifeBarEnemie` (`WidgetComponent.GetWidget` (`self.LifeBar`))))
  (`ProgressBar.SetFillColorAndOpacity` (`/Game/UI/WBP_LifeBarEnemie.healthBar` _aswbp_life_bar_enemie) (struct :`R` 0.075955 :`G` 0.644628 :`B` 0.729167 :`A` 1.0)))

(event `self.ReceiveTick`
  (params (DeltaSeconds :type "Float (single-precision)"))
  (bind _returnvalue (`self.GetHealthPercent`))
  (bind _aswbp_life_bar_enemie (cast `/Game/UI/WBP_LifeBarEnemie` (`WidgetComponent.GetWidget` (`self.LifeBar`))))
  (`ProgressBar.SetPercent` (`/Game/UI/WBP_LifeBarEnemie.healthBar` _aswbp_life_bar_enemie) _returnvalue)
  (if (== _returnvalue 0.0)
    (`SceneComponent.SetVisibility` (`self.LifeBar`) false false)))

(event `self.ReceivePossessed`
  (params (NewController :type "Controller Object Reference"))
  (`SceneComponent.SetVisibility` (`self.SM_Wraith_Drone_ElectroField`) false false))

(event `self.ActiveShell`
  (`SceneComponent.SetVisibility` (`self.SM_Wraith_Drone_ElectroField`) true false)
  (`KismetSystemLibrary.Delay` 5.0)
  (`self.RemoveShell`))

(event `RemoveShell`
  (`SceneComponent.SetVisibility` (`self.SM_Wraith_Drone_ElectroField`) false false)
  (if (`self.ActorHasTag` "Shell")
    (`KismetArrayLibrary.Array_RemoveItem` (`self.Tags`) "Shell")))

(fn `UserConstructionScript`)