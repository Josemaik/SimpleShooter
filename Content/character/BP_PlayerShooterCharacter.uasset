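; Player shooter character Blueprint that handles camera switching and relays gameplay events to the HUD.
; SwitchCam flip-flops between first-person and default cameras, storing the choice so HandleKillCamera can restore it after the kill camera.
; Potion and mission events cast through player controller 0 to WBP_HUD, with missions picked by comparing stringified numbers.
; Other events toggle the pass panel and notify BP_Rifle of enemy hits; an intro sound node is unconnected.
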(event `self.ReceiveBeginPlay`
  (`parent.ReceiveBeginPlay`))

(event `self.SwitchCam`
  (`/Engine/EditorBlueprintResources/StandardMacros.FlipFlop`
    (:`A`
      (`ActorComponent.SetActive` (`self.FirstPersonCamera_0`) true false)
      (`ActorComponent.SetActive` (`self.Camera`) false false)
      (set `self.bUseControllerRotationYaw` true)
      (set `self.switch_camera` true))
    (:`B`
      (`ActorComponent.SetActive` (`self.FirstPersonCamera_0`) false false)
      (`ActorComponent.SetActive` (`self.Camera`) true false)
      (set `self.bUseControllerRotationYaw` true)
      (set `self.switch_camera` false))))

(event `self.HandleKillCamera`
  (params (mode :type Boolean))
  (bind _switch_camera (`self.switch_camera`))
  (if mode
    (if _switch_camera
      (`ActorComponent.SetActive` (`self.FirstPersonCamera_0`) false false)
      (`ActorComponent.SetActive` (`self.KillCamera`) true false)
      (else
        (`ActorComponent.SetActive` (`self.FirstPersonCamera_0`) false false)
        (`ActorComponent.SetActive` (`self.Camera`) false false)
        (`ActorComponent.SetActive` (`self.KillCamera`) true false)))
    (else
      (if _switch_camera
        (`ActorComponent.SetActive` (`self.FirstPersonCamera_0`) true false)
        (else
          (`ActorComponent.SetActive` (`self.Camera`) true false)))
      (`ActorComponent.SetActive` (`self.KillCamera`) false false))))

(event `self.GetMaxPotions`
  (`KismetSystemLibrary.PrintString` "Event get max potions")
  (bind _asshooter_player_controller (cast `ShooterPlayerController` (`GameplayStatics.GetPlayerController` 0)))
  (bind _aswbp_hud (cast `/Game/UI/WBP_HUD` (`ShooterPlayerController.HUD` _asshooter_player_controller)))
  (`/Game/UI/WBP_HUD.GetMaxPotions` _aswbp_hud))

(event `self.DeleteCurePotion`
  (params (newcurrentpotion :type Integer))
  (bind _asshooter_player_controller (cast `ShooterPlayerController` (`GameplayStatics.GetPlayerController` 0)))
  (bind _aswbp_hud (cast `/Game/UI/WBP_HUD` (`ShooterPlayerController.HUD` _asshooter_player_controller)))
  (`/Game/UI/WBP_HUD.DeletePotion` _aswbp_hud newcurrentpotion))

(event `self.NewMision`
  (params (newcurrentpotion :type Name))
  (bind _returnvalue (`KismetStringLibrary.Conv_NameToString` newcurrentpotion))
  (`KismetSystemLibrary.PrintString` _returnvalue)
  (bind _asshooter_player_controller (cast `ShooterPlayerController` (`GameplayStatics.GetPlayerController` 0)))
  (bind _aswbp_hud (cast `/Game/UI/WBP_HUD` (`ShooterPlayerController.HUD` _asshooter_player_controller))
    (:`then`
      (if (`KismetStringLibrary.EqualEqual_StrStr` _returnvalue "3")
        (`/Game/UI/WBP_HUD.Mision_hack_main_panel` _aswbp_hud)
        (elif (`KismetStringLibrary.EqualEqual_StrStr` _returnvalue "2")
          (`/Game/UI/WBP_HUD.Mision_unlock_door` _aswbp_hud)
          (elif (`KismetStringLibrary.EqualEqual_StrStr` _returnvalue "1")
            (`/Game/UI/WBP_HUD.Key_pista` _aswbp_hud)
            (else
              (`/Game/UI/WBP_HUD.Mision_Find_key` _aswbp_hud))))))
    (:`CastFailed`
      (`KismetSystemLibrary.PrintString` "failed"))))

(event `hidde_pass_panel`
  (`SceneComponent.SetVisibility` (`self.Pass_panel`) false false))

(event `pass_panel_tablet`
  (`SceneComponent.SetVisibility` (`self.Pass_panel`) true false))

(event `self.Takedamage`
  (if (`self.ActorHasTag` "Player")
    (bind _asbp_rifle (cast `/Game/guns/BP_Rifle` (`self.GetCurrentGun`)))
    (`/Game/guns/BP_Rifle.HitbyEnemy` _asbp_rifle)))

(fn `UserConstructionScript`
  (`parent.UserConstructionScript`))