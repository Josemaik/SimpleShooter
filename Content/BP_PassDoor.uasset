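; BP_PassDoor is a passcode door that shows the HUD's pass-entry panel while a Player-tagged actor is in its trigger.
; BeginPlay links the Mover to the Trigger component.
; Trigger overlaps reach WBP_HUD through player controller 0, toggling PanelEnterPass visibility and swapping a material slot on the Pad.
; This graph contains no pass validation or direct door movement, only the panel and pad feedback.
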(event `self.ReceiveBeginPlay`
  (`TriggerComponent.SetMover` (`self.Trigger`) (`self.Mover`)))

(event `self.Trigger.OnComponentBeginOverlap`
  (params (OverlappedComponent :type "PrimitiveComponent Object Reference") (OtherActor :type "Actor Object Reference") (OtherComp :type "PrimitiveComponent Object Reference") (OtherBodyIndex :type Integer) (bFromSweep :type Boolean) (SweepResult :type "HitResult Structure (by ref)"))
  (`KismetSystemLibrary.PrintString` "overlaping")
  (if (`self.ActorHasTag` OtherActor "Player")
    (bind _asbp_shooter_player_controller (cast `/Game/BP_ShooterPlayerController` (`GameplayStatics.GetPlayerController` 0)))
    (bind _aswbp_hud (cast `/Game/UI/WBP_HUD` (`ShooterPlayerController.HUD` _asbp_shooter_player_controller)))
    (`/Engine/EditorBlueprintResources/StandardMacros.IsValid` _aswbp_hud
      (:`Is Valid`
        (`Widget.SetVisibility` (`/Game/UI/WBP_HUD.Panel_EnterPass` _aswbp_hud) "Visible")
        (`PrimitiveComponent.SetMaterial` (`self.pad`) 1 "/Game/AssetPacks/ModularSciFiSeason1/StarterBundle/ModularScifiHallways/Materials/M_Base_Wires.M_Base_Wires")))))

(event `self.Trigger.OnComponentEndOverlap`
  (params (OverlappedComponent :type "PrimitiveComponent Object Reference") (OtherActor :type "Actor Object Reference") (OtherComp :type "PrimitiveComponent Object Reference") (OtherBodyIndex :type Integer))
  (if (`self.ActorHasTag` OtherActor "Player")
    (bind _asbp_shooter_player_controller (cast `/Game/BP_ShooterPlayerController` (`GameplayStatics.GetPlayerController` 0)))
    (bind _aswbp_hud (cast `/Game/UI/WBP_HUD` (`ShooterPlayerController.HUD` _asbp_shooter_player_controller)))
    (`/Engine/EditorBlueprintResources/StandardMacros.IsValid` _aswbp_hud
      (:`Is Valid`
        (`Widget.SetVisibility` (`/Game/UI/WBP_HUD.Panel_EnterPass` _aswbp_hud) "Hidden")
        (`PrimitiveComponent.SetMaterial` (`self.pad`) 1 "/Game/AssetPacks/ModularSciFiSeason1/StarterBundle/ModularScifiHallways/Materials/M_UI_Parent.M_UI_Parent")))))

(fn `UserConstructionScript`)