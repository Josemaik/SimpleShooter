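; Elevator actor that links a trigger to a mover component and advances the player's mission.
; On BeginPlay it passes Mover to Trigger through SetMover; the movement logic itself lives outside this graph.
; When a Player-tagged actor overlaps Trigger, it calls NewMision on the player's BP_ShooterCharacter, choosing mission "1" or "2" by whether the trigger carries the Elevator tag.
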(event `self.ReceiveBeginPlay`
  (`TriggerComponent.SetMover` (`self.Trigger`) (`self.Mover`)))

(event `OnActorBeginOverlap_Event`
  (params (OverlappedActor :type "Actor Object Reference") (OtherActor :type "Actor Object Reference")))

(event `self.Trigger.OnComponentBeginOverlap`
  (params (OverlappedComponent :type "PrimitiveComponent Object Reference") (OtherActor :type "Actor Object Reference") (OtherComp :type "PrimitiveComponent Object Reference") (OtherBodyIndex :type Integer) (bFromSweep :type Boolean) (SweepResult :type "HitResult Structure (by ref)"))
  (if (`self.ActorHasTag` OtherActor "Player")
    (if (`ActorComponent.ComponentHasTag` OverlappedComponent "Elevator")
      (bind _asbp_shooter_character (cast `/Game/character/BP_ShooterCharacter` (`GameplayStatics.GetPlayerPawn` 0)))
      (`ShooterCharacter.NewMision` _asbp_shooter_character "1")
      (else
        (bind _asbp_shooter_character_2 (cast `/Game/character/BP_ShooterCharacter` (`GameplayStatics.GetPlayerPawn` 0)))
        (`ShooterCharacter.NewMision` _asbp_shooter_character_2 "2")))))

(fn `UserConstructionScript`)