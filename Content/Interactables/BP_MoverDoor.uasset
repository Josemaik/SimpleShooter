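; BP_MoverDoor is an interactable door built from a Trigger component and a Mover component.
; BeginPlay passes the Mover to the Trigger through SetMover, leaving the movement logic to those components.
; The Blueprint itself plays a door-opening sound at the actor's location when a Player-tagged actor overlaps the Trigger, unless Mover's EndMove returns true or the door is tagged PickGunDoor.
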(event `self.ReceiveBeginPlay`
  (`TriggerComponent.SetMover` (`self.Trigger`) (`self.Mover`)))

(event `self.Trigger.OnComponentBeginOverlap`
  (params (OverlappedComponent :type "PrimitiveComponent Object Reference") (OtherActor :type "Actor Object Reference") (OtherComp :type "PrimitiveComponent Object Reference") (OtherBodyIndex :type Integer) (bFromSweep :type Boolean) (SweepResult :type "HitResult Structure (by ref)"))
  (if (and (`self.ActorHasTag` OtherActor "Player") (not (`Mover.EndMove` (`self.Mover`))) (not (`self.ActorHasTag` "PickGunDoor")))
    (`GameplayStatics.PlaySoundAtLocation` "/Game/SFX/SW_doorOpening.SW_doorOpening" (`self.K2_GetActorLocation`) (struct) 1.0 1.0 0.0 null null null null)))

(fn `UserConstructionScript`)