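; Shotgun Blueprint that drives HUD feedback for pickup proximity and damage numbers.
; Its collision sphere shows or hides the HUD pickup panel as a Player-tagged actor enters or leaves.
; DrawDamageTaken writes the damage to the HUD, plays one of three random hit animations and hides the text when it finishes.
; Both paths reach WBP_HUD through the first player controller; disconnected debug nodes remain in the graph.
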(event `self.ReceiveBeginPlay`)

(event `self.SphereCollision.OnComponentBeginOverlap`
  (params (OverlappedComponent :type "PrimitiveComponent Object Reference") (OtherActor :type "Actor Object Reference") (OtherComp :type "PrimitiveComponent Object Reference") (OtherBodyIndex :type Integer) (bFromSweep :type Boolean) (SweepResult :type "HitResult Structure (by ref)"))
  (if (`self.ActorHasTag` OtherActor "Player")
    (bind _asbp_shooter_player_controller (cast `/Game/BP_ShooterPlayerController` (`GameplayStatics.GetPlayerController` 0)))
    (bind _aswbp_hud (cast `/Game/UI/WBP_HUD` (`ShooterPlayerController.HUD` _asbp_shooter_player_controller)))
    (`/Engine/EditorBlueprintResources/StandardMacros.IsValid` _aswbp_hud
      (:`Is Valid`
        (`Widget.SetVisibility` (`/Game/UI/WBP_HUD.PickPanel` _aswbp_hud) "Visible")))))

(event `self.SphereCollision.OnComponentEndOverlap`
  (params (OverlappedComponent :type "PrimitiveComponent Object Reference") (OtherActor :type "Actor Object Reference") (OtherComp :type "PrimitiveComponent Object Reference") (OtherBodyIndex :type Integer))
  (if (`self.ActorHasTag` OtherActor "Player")
    (bind _asbp_shooter_player_controller (cast `/Game/BP_ShooterPlayerController` (`GameplayStatics.GetPlayerController` 0)))
    (bind _aswbp_hud (cast `/Game/UI/WBP_HUD` (`ShooterPlayerController.HUD` _asbp_shooter_player_controller)))
    (`/Engine/EditorBlueprintResources/StandardMacros.IsValid` _aswbp_hud
      (:`Is Valid`
        (`Widget.SetVisibility` (`/Game/UI/WBP_HUD.PickPanel` _aswbp_hud) "Hidden")))))

(event `self.DrawDamageTaken`
  (params (damage :type "Float (single-precision)"))
  (bind _asshooter_player_controller (cast `ShooterPlayerController` (`GameplayStatics.GetPlayerController` 0)))
  (bind _aswbp_hud (cast `/Game/UI/WBP_HUD` (`ShooterPlayerController.HUD` _asshooter_player_controller)))
  (`/Engine/EditorBlueprintResources/StandardMacros.IsValid` _aswbp_hud
    (:`Is Valid`
      (bind _damagetaken (`/Game/UI/WBP_HUD.damagetaken` _aswbp_hud))
      (`TextBlock.SetText` _damagetaken (`KismetTextLibrary.Conv_DoubleToText` damage "HalfToEven"))
      (`Widget.SetVisibility` _damagetaken "Visible")
      (switch `int` (`KismetMathLibrary.RandomInteger` 3)
        (:`0`
          (bind _hiting (`/Game/UI/WBP_HUD.hiting` _aswbp_hud))
          (`UserWidget.PlayAnimation` _aswbp_hud _hiting 0.0 1 "Forward" 1.0 false)
          (`UserWidget.BindToAnimationFinished` _aswbp_hud _hiting (delegate `CustomEvent`)))
        (:`1`
          (bind _hiting_0 (`/Game/UI/WBP_HUD.hiting_0` _aswbp_hud))
          (`UserWidget.PlayAnimation` _aswbp_hud _hiting_0 0.0 1 "Forward" 1.0 false)
          (`UserWidget.BindToAnimationFinished` _aswbp_hud _hiting_0 (delegate `CustomEvent`)))
        (:`2`
          (bind _hiting_1 (`/Game/UI/WBP_HUD.hiting_1` _aswbp_hud))
          (`UserWidget.PlayAnimation` _aswbp_hud _hiting_1 0.0 1 "Forward" 1.0 false)
          (`UserWidget.BindToAnimationFinished` _aswbp_hud _hiting_1 (delegate `CustomEvent`)))))))

(event `CustomEvent`
  (`Widget.SetVisibility` (`/Game/UI/WBP_HUD.damagetaken` (stale `self.DrawDamageTaken` _aswbp_hud)) "Hidden"))

(fn `UserConstructionScript`)